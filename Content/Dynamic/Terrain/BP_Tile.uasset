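; BP_Tile is one segment of an infinite terrain that populates itself on BeginPlay with containers, boxes, canisters, rocks and sandbags through PlaceActors.
; Its barrier starts locked in red, turns passable green while the player is in LockingVolume, and relocks on exit as the game mode spawns another tile.
; GetAttachLocation exposes the Arrow transform as an attach point, and the tile destroys itself when the player enters DestroyVolume.
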(event OnComponentBeginOverlap(LockingVolume)
  (params (OverlappedComponent :type Primitive%20Component%20Object%20Reference) (OtherActor :type Actor%20Object%20Reference) (OtherComp :type Primitive%20Component%20Object%20Reference) (OtherBodyIndex :type Integer) (bFromSweep :type Boolean) (SweepResult :type Hit%20Result%20Structure%20%28by%20ref%29))
  (Utilities|IsPlayerActor OtherActor)
  (CallFunction|UnlockWall))

(event OnComponentEndOverlap(LockingVolume)
  (params (OverlappedComponent :type Primitive%20Component%20Object%20Reference) (OtherActor :type Actor%20Object%20Reference) (OtherComp :type Primitive%20Component%20Object%20Reference) (OtherBodyIndex :type Integer))
  (Utilities|IsPlayerActor OtherActor)
  (CallFunction|LockWall)
  (bind _asinfinite_terrain_game_mode (Utilities|Casting|CastToInfiniteTerrainGameMode (Game|GetGameMode)))
  (Default|SpawnTile _asinfinite_terrain_game_mode))

(event OnComponentBeginOverlap(DestroyVolume)
  (params (OverlappedComponent :type Primitive%20Component%20Object%20Reference) (OtherActor :type Actor%20Object%20Reference) (OtherComp :type Primitive%20Component%20Object%20Reference) (OtherBodyIndex :type Integer) (bFromSweep :type Boolean) (SweepResult :type Hit%20Result%20Structure%20%28by%20ref%29))
  (Utilities|IsPlayerActor OtherActor)
  (Actor|DestroyActor))

(event EventBeginPlay
  (CallFunction|LockWall)
  (Class|Tile|PlaceActors "/Game/Dynamic/Terrain/Props/BP_Container_01.BP_Container_01_C" 1 3 4e+02 1.0 1.0)
  (Class|Tile|PlaceActors "/Game/Dynamic/Terrain/Props/BP_Box_01.BP_Box_01_C" 2 4 1e+02 1.0 1.0)
  (Class|Tile|PlaceActors "/Game/Dynamic/Terrain/Props/BP_Canister_01.BP_Canister_01_C" 1 7 5e+01 1.0 1.0)
  (Class|Tile|PlaceActors "/Game/Dynamic/Terrain/Props/BP_Rock_01.BP_Rock_01_C" 1 4 1.5e+02 1.0 5.0)
  (Class|Tile|PlaceActors "/Game/Dynamic/Terrain/Props/BP_Rock_02.BP_Rock_02_C" 1 4 2.5e+02 1.0 5.0)
  (Class|Tile|PlaceActors "/Game/Dynamic/Terrain/Props/BP_Rock_03.BP_Rock_03_C" 1 4 2.5e+02 1.0 5.0)
  (Class|Tile|PlaceActors "/Game/Dynamic/Terrain/Props/BP_Sandbags_01.BP_Sandbags_01_C" 1 3 2.5e+02 1.0 1.0))

(fn ConstructionScript)

(fn GetAttachLocation
  (return (Transformation|GetWorldTransform (Variables|Default|GetArrow))))

(fn UnlockWall
  (bind _barrier (Variables|Default|GetBarrier))
  (Collision|SetCollisionEnabled _barrier "NoCollision")
  (Rendering|Material|SetMaterial _barrier 0 "/Game/Dynamic/Terrain/MI_Barrier_Green.MI_Barrier_Green"))

(fn LockWall
  (bind _barrier (Variables|Default|GetBarrier))
  (Collision|SetCollisionEnabled _barrier "QueryAndPhysics")
  (Rendering|Material|SetMaterial _barrier 0 "/Game/Dynamic/Terrain/MI_Barrier_Red.MI_Barrier_Red"))